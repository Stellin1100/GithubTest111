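; Zombie enemy AI that roams the navmesh at random and chases the player when PawnSensing spots them, growling once it reaches them.
; A Tick-driven Delay throttles wandering, which a CanSeePlayer flag suspends during sight chases.
; Bullet overlaps reduce health, triggering blood and pursuit, or a death animation, screen widget and delayed destruction at zero.
; A sphere overlap damages the player through TakeDamage5.
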(event OnSeePawn(PawnSensing)
  (params (Pawn :type Pawn%20Object%20Reference))
  (if (not (Variables|Default|GetCanSeePlayer))
    (bind _asthird_person_character (Utilities|Casting|CastToThirdPersonCharacter (Game|GetPlayerCharacter 0)))
    (Variables|Default|SetCanSeePlayer true)
    (AI|AIMoveTo self "0, 0, 0" _asthird_person_character 5.0 false
      (:OnSuccess
        (Audio|SpawnSoundatLocation "/Game/Group-Of-Zombies-Growling-A1-www_fesliyanstudios_com.Group-Of-Zombies-Growling-A1-www_fesliyanstudios_com" "0, 0, 0" "0, 0, 0" 1.0 1.0 0.0 0 0))
      (:OnFail
        _))
    (Variables|Default|SetCanSeePlayer false)))

(event OnComponentBeginOverlap(Sphere)
  (params (OverlappedComponent :type Primitive%20Component%20Object%20Reference) (OtherActor :type Actor%20Object%20Reference) (OtherComp :type Primitive%20Component%20Object%20Reference) (OtherBodyIndex :type Integer) (bFromSweep :type Boolean) (SweepResult :type Hit%20Result%20Structure%20%28by%20ref%29))
  (bind _asthird_person_character (Utilities|Casting|CastToThirdPersonCharacter OtherActor))
  (Default|TakeDamage5% _asthird_person_character))

(event EventTick
  (params (DeltaSeconds :type Float%20%28single-precision%29))
  (Utilities|FlowControl|Delay 2.0)
  (if (not (Variables|Default|GetCanSeePlayer))
    (AI|AIMoveTo self (.RandomLocation (Class|NavigationSystemV1|GetRandomPointinNavigableRadius (Transformation|GetActorLocation) 3e+03 0 0)) 0 5.0 false)))

(event Collision|EventActorBeginOverlap
  (params (OtherActor :type Actor%20Object%20Reference))
  (bind _asbp_bullet (Utilities|Casting|CastToBP_Bullet OtherActor))
  (Variables|Default|Sethealth (- (Variables|Default|Gethealth) 0.1))
  (if (<= (Variables|Default|Gethealth) 0.0)
    (Components|Animation|PlayAnimation (Variables|Character|GetMesh) "/Game/anim/zombi/animation/Zombie_Death.Zombie_Death" false)
    (bind _returnvalue (UserInterface|CreateWidget "/Game/111/WBP_efect.WBP_efect_C"))
    (UserInterface|Viewport|AddtoViewport _returnvalue 0)
    (Pawn|Components|CharacterMovement|DisableMovement (Variables|Character|GetCharacterMovement))
    (Utilities|FlowControl|Delay 4.0)
    (Actor|DestroyActor)
    (else
      (Effects|SpawnEmitteratLocation "/Game/Realistic_Starter_VFX_Pack_Vol2/Particles/Blood/P_Blood_Splat_Cone.P_Blood_Splat_Cone" (Transformation|GetActorLocation _asbp_bullet) "0, 0, 0" "1.000000,1.000000,1.000000" true "AutoRelease")
      (bind _asthird_person_character (Utilities|Casting|CastToThirdPersonCharacter (Game|GetPlayerCharacter 0)))
      (AI|AIMoveTo self "0, 0, 0" _asthird_person_character 5.0 false))))

(fn ConstructionScript)